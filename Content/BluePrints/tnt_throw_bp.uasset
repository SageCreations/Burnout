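; Thrown TNT projectile actor with a Paper2D sprite that flies horizontally in the player's facing direction.
; On BeginPlay it copies PlayerDirection from the player character, cast to PlayerController_BP.
; Tick sweeps it a fixed step along local X, forward or backward by that flag, without delta-time scaling.
; When the sprite overlaps an actor tagged Door1, it prints a debug string and destroys itself after a brief delay.
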(event `self.ReceiveBeginPlay`
  (bind _asplayer_controller_bp (cast `/Game/BluePrints/PlayerController_BP` (`GameplayStatics.GetPlayerCharacter` 0)))
  (set `self.direction` (`/Game/BluePrints/PlayerController_BP.playerDirection` _asplayer_controller_bp)))

(event `self.ReceiveTick`
  (params (DeltaSeconds :type "Float (single-precision)"))
  (if (`self.direction`)
    (`self.K2_AddActorLocalTransform` (`KismetMathLibrary.MakeTransform` (20.0 0.0 0.0)) true)
    (else
      (`self.K2_AddActorLocalTransform` (`KismetMathLibrary.MakeTransform` (-20.0 0.0 0.0)) true))))

(event `self.PaperSprite.OnComponentBeginOverlap`
  (params (OverlappedComponent :type "PrimitiveComponent Object Reference") (OtherActor :type "Actor Object Reference") (OtherComp :type "PrimitiveComponent Object Reference") (OtherBodyIndex :type Integer) (bFromSweep :type Boolean) (SweepResult :type "HitResult Structure (by ref)"))
  (if (`self.ActorHasTag` OtherActor "Door1")
    (`KismetSystemLibrary.PrintString` "Hello")
    (`KismetSystemLibrary.Delay` 0.05)
    (`self.K2_DestroyActor`)))

(fn `UserConstructionScript`)