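; CheckPoint_bp is a checkpoint actor that sets the player's spawn position and lights a fire when reached.
; On BeginPlay it writes a hard-coded default spawn position to the player character, cast to PlayerController_BP, and hides the FireFrame and PointLight.
; Any overlap with its Box sets that spawn position to the checkpoint's location and shows both components, without checking which actor overlapped.
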(event `self.ReceiveBeginPlay`
  (bind _asplayer_controller_bp (cast `/Game/BluePrints/PlayerController_BP` (`GameplayStatics.GetPlayerCharacter` 0)))
  (set `/Game/BluePrints/PlayerController_BP.Spawnposition` (350.0 0.0 -3857.498535) _asplayer_controller_bp)
  (`SceneComponent.SetVisibility` (`self.fire_frame`) false false)
  (`SceneComponent.SetVisibility` (`self.PointLight`) false false))

(event `self.Box.OnComponentBeginOverlap`
  (params (OverlappedComponent :type "PrimitiveComponent Object Reference") (OtherActor :type "Actor Object Reference") (OtherComp :type "PrimitiveComponent Object Reference") (OtherBodyIndex :type Integer) (bFromSweep :type Boolean) (SweepResult :type "HitResult Structure (by ref)"))
  (bind _asplayer_controller_bp (cast `/Game/BluePrints/PlayerController_BP` (`GameplayStatics.GetPlayerCharacter` 0)))
  (set `/Game/BluePrints/PlayerController_BP.Spawnposition` (`self.K2_GetActorLocation`) _asplayer_controller_bp)
  (`SceneComponent.SetVisibility` (`self.fire_frame`) true false)
  (`SceneComponent.SetVisibility` (`self.PointLight`) true false))

(fn `UserConstructionScript`)