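; Trigger actor that reveals a background fire element when the player reaches it.
; On BeginPlay it hides the FireFrame component through both hidden-in-game and visibility flags, without propagating to children.
; When an actor tagged Player begins overlapping the Box component, both flags are flipped to show FireFrame.
; No end-overlap logic exists, so the frame stays visible once revealed.
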(event `self.ReceiveBeginPlay`
  (`SceneComponent.SetHiddenInGame` (`self.fire_frame`) true false)
  (`SceneComponent.SetVisibility` (`self.fire_frame`) false false))

(event `self.Box.OnComponentBeginOverlap`
  (params (OverlappedComponent :type "PrimitiveComponent Object Reference") (OtherActor :type "Actor Object Reference") (OtherComp :type "PrimitiveComponent Object Reference") (OtherBodyIndex :type Integer) (bFromSweep :type Boolean) (SweepResult :type "HitResult Structure (by ref)"))
  (if (`self.ActorHasTag` OtherActor "Player")
    (`SceneComponent.SetHiddenInGame` (`self.fire_frame`) false false)
    (`SceneComponent.SetVisibility` (`self.fire_frame`) true false)))

(fn `UserConstructionScript`)