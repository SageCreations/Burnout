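; Spawnable barrel hazard that kills the player on contact, judging by its name and overlap logic.
; When its RenderComponent begins overlapping a "Player"-tagged actor, it sets PlayerDead on the player character, which is cast to PlayerController_BP despite that class's name.
; Tick polls the component's overlap and, once PlayerDead is set, destroys the barrel after a short delay.
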(event `self.ReceiveTick`
  (params (DeltaSeconds :type "Float (single-precision)"))
  (if (`PrimitiveComponent.IsOverlappingActor` (`self.RenderComponent`) null)
    (bind _asplayer_controller_bp (cast `/Game/BluePrints/PlayerController_BP` (`GameplayStatics.GetPlayerCharacter` 0)))
    (if (`/Game/BluePrints/PlayerController_BP.playerDead` _asplayer_controller_bp)
      (`KismetSystemLibrary.Delay` 0.2)
      (`self.K2_DestroyActor`))))

(event `self.RenderComponent.OnComponentBeginOverlap`
  (params (OverlappedComponent :type "PrimitiveComponent Object Reference") (OtherActor :type "Actor Object Reference") (OtherComp :type "PrimitiveComponent Object Reference") (OtherBodyIndex :type Integer) (bFromSweep :type Boolean) (SweepResult :type "HitResult Structure (by ref)"))
  (if (`self.ActorHasTag` OtherActor "Player")
    (bind _asplayer_controller_bp (cast `/Game/BluePrints/PlayerController_BP` (`GameplayStatics.GetPlayerCharacter` 0)))
    (set `/Game/BluePrints/PlayerController_BP.playerDead` true _asplayer_controller_bp)))

(fn `UserConstructionScript`)