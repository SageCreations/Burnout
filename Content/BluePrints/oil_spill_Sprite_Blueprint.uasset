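; Oil spill hazard actor that marks the player as standing on oil while its Box trigger is overlapped.
; Begin and end overlap events set and clear OnOil on the player character, cast to PlayerController_BP, without checking which actor triggered them.
; Tick prints whether the box overlaps the player each frame as debug output.
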(event `self.ReceiveTick`
  (params (DeltaSeconds :type "Float (single-precision)"))
  (bind _asplayer_controller_bp (cast `/Game/BluePrints/PlayerController_BP` (`GameplayStatics.GetPlayerCharacter` 0)))
  (`KismetSystemLibrary.PrintString` (`KismetStringLibrary.Conv_BoolToString` (`PrimitiveComponent.IsOverlappingActor` (`self.Box`) _asplayer_controller_bp))))

(event `self.Box.OnComponentBeginOverlap`
  (params (OverlappedComponent :type "PrimitiveComponent Object Reference") (OtherActor :type "Actor Object Reference") (OtherComp :type "PrimitiveComponent Object Reference") (OtherBodyIndex :type Integer) (bFromSweep :type Boolean) (SweepResult :type "HitResult Structure (by ref)"))
  (bind _asplayer_controller_bp (cast `/Game/BluePrints/PlayerController_BP` (`GameplayStatics.GetPlayerCharacter` 0)))
  (set `/Game/BluePrints/PlayerController_BP.onOil` true _asplayer_controller_bp))

(event `self.Box.OnComponentEndOverlap`
  (params (OverlappedComponent :type "PrimitiveComponent Object Reference") (OtherActor :type "Actor Object Reference") (OtherComp :type "PrimitiveComponent Object Reference") (OtherBodyIndex :type Integer))
  (bind _asplayer_controller_bp (cast `/Game/BluePrints/PlayerController_BP` (`GameplayStatics.GetPlayerCharacter` 0)))
  (set `/Game/BluePrints/PlayerController_BP.onOil` false _asplayer_controller_bp))

(fn `UserConstructionScript`)