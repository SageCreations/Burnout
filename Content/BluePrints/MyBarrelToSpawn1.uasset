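; A spawnable barrel hazard that moves horizontally and kills the player on touch.
; Each tick it shifts its render component along local X, with the Rolly flag choosing the direction.
; Overlapping an actor tagged Player sets PlayerDead on the player character, cast to PlayerController_BP.
; Tick also polls that flag and destroys the barrel after a short delay once the player is dead.
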(event `self.ReceiveBeginPlay`)

(event `self.ReceiveTick`
  (params (DeltaSeconds :type "Float (single-precision)"))
  (if (`self.rolly`)
    (`SceneComponent.K2_AddLocalTransform` (`self.RenderComponent`) (`KismetMathLibrary.MakeTransform` (-5.0 0.0 0.0) (struct) (2.0 1.0 2.0)) false false)
    (else
      (`SceneComponent.K2_AddLocalTransform` (`self.RenderComponent`) (`KismetMathLibrary.MakeTransform` (5.0 0.0 0.0) (struct) (2.0 1.0 2.0)) false false)))
  (bind _asplayer_controller_bp (cast `/Game/BluePrints/PlayerController_BP` (`GameplayStatics.GetPlayerCharacter` 0)))
  (if (`/Game/BluePrints/PlayerController_BP.playerDead` _asplayer_controller_bp)
    (`KismetSystemLibrary.Delay` 0.2)
    (`self.K2_DestroyActor`)))

(event `self.RenderComponent.OnComponentBeginOverlap`
  (params (OverlappedComponent :type "PrimitiveComponent Object Reference") (OtherActor :type "Actor Object Reference") (OtherComp :type "PrimitiveComponent Object Reference") (OtherBodyIndex :type Integer) (bFromSweep :type Boolean) (SweepResult :type "HitResult Structure (by ref)"))
  (if (`self.ActorHasTag` OtherActor "Player")
    (bind _asplayer_controller_bp (cast `/Game/BluePrints/PlayerController_BP` (`GameplayStatics.GetPlayerCharacter` 0)))
    (set `/Game/BluePrints/PlayerController_BP.playerDead` true _asplayer_controller_bp)))

(fn `UserConstructionScript`)