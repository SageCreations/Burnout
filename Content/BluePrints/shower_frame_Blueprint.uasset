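; Shower flipbook actor that acts as a level goal, putting out the player's fire and leading to the win menu.
; It starts hidden; a "Player"-tagged overlap on its Box plays the shower sound, reveals the animation and, after a short delay, swaps flipbooks.
; It then hides Fire and FireLight on the player character, cast to PlayerController_BP, and opens Win_menu after another delay.
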(event `self.ReceiveBeginPlay`
  (`SceneComponent.SetHiddenInGame` (`self.RenderComponent`) true false))

(event `self.Box.OnComponentBeginOverlap`
  (params (OverlappedComponent :type "PrimitiveComponent Object Reference") (OtherActor :type "Actor Object Reference") (OtherComp :type "PrimitiveComponent Object Reference") (OtherBodyIndex :type Integer) (bFromSweep :type Boolean) (SweepResult :type "HitResult Structure (by ref)"))
  (if (`self.ActorHasTag` OtherActor "Player")
    (`GameplayStatics.PlaySound2D` "/Game/Assets/Sounds/shower_sfx.shower_sfx" 1.0 1.0 0.3 null null)
    (`PaperFlipbookComponent.PlayFromStart` (`self.RenderComponent`))
    (`SceneComponent.SetHiddenInGame` (`self.RenderComponent`) false false)
    (`KismetSystemLibrary.Delay` 0.3)
    (`PaperFlipbookComponent.SetFlipbook` (`self.RenderComponent`) "/Game/Assets/Shower/shower_frame1.shower_frame1")
    (bind _asplayer_controller_bp (cast `/Game/BluePrints/PlayerController_BP` (`GameplayStatics.GetPlayerCharacter` 0)))
    (`SceneComponent.SetVisibility` (`/Game/BluePrints/PlayerController_BP.Fire` _asplayer_controller_bp) false false)
    (`SceneComponent.SetVisibility` (`/Game/BluePrints/PlayerController_BP.FireLight` _asplayer_controller_bp) false false)
    (`KismetSystemLibrary.Delay` 1.0)
    (`GameplayStatics.OpenLevelBySoftObjectPtr` "/Game/win_menu.win_menu")))

(fn `UserConstructionScript`)