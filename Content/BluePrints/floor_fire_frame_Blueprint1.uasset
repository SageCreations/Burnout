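; Floor fire hazard that stays hidden until a Player-tagged actor enters its Box, then ignites and can kill the player.
; The overlap picks a random animation frame and, after short delays, shows the sprite and light and arms the fire.
; Tick sets PlayerDead on the player character inside DeathBox while armed.
; Outside DeathBox, a dead player makes Tick hide and disarm the fire.
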(event `self.ReceiveBeginPlay`
  (`SceneComponent.SetVisibility` (`self.PointLight`) false false)
  (`SceneComponent.SetVisibility` (`self.RenderComponent`) false false))

(event `self.Box.OnComponentBeginOverlap`
  (params (OverlappedComponent :type "PrimitiveComponent Object Reference") (OtherActor :type "Actor Object Reference") (OtherComp :type "PrimitiveComponent Object Reference") (OtherBodyIndex :type Integer) (bFromSweep :type Boolean) (SweepResult :type "HitResult Structure (by ref)"))
  ;[1 1 1] Collision to catch oil on fire
  (if (`self.ActorHasTag` OtherActor "Player")
    (`PaperFlipbookComponent.SetPlaybackPositionInFrames` (`self.RenderComponent`) (`KismetMathLibrary.RandomInteger` 8) false)
    (`KismetSystemLibrary.Delay` 0.2)
    (`SceneComponent.SetVisibility` (`self.RenderComponent`) true false)
    (`SceneComponent.SetVisibility` (`self.PointLight`) true false)
    (`KismetSystemLibrary.Delay` 0.2)
    (set `self.isFireVisible` true)))

(event `self.ReceiveTick`
  (params (DeltaSeconds :type "Float (single-precision)"))
  ;[1 1 1] checks for deathbox and player overlap
  (bind _asplayer_controller_bp (cast `/Game/BluePrints/PlayerController_BP` (`GameplayStatics.GetPlayerCharacter` 0)))
  (if (`PrimitiveComponent.IsOverlappingActor` (`self.DeathBox`) _asplayer_controller_bp)
    ;[1 1 1] Sets player dead true
    (if (`self.isFireVisible`)
      (set `/Game/BluePrints/PlayerController_BP.playerDead` true _asplayer_controller_bp))
    (else
      ;[1 1 1] Resets fire anim if player dies
      (bind _asplayer_controller_bp_2 (cast `/Game/BluePrints/PlayerController_BP` (`GameplayStatics.GetPlayerCharacter` 0)))
      (if (`/Game/BluePrints/PlayerController_BP.playerDead` _asplayer_controller_bp_2)
        (`PaperFlipbookComponent.SetPlaybackPositionInFrames` (`self.RenderComponent`) (`KismetMathLibrary.RandomInteger` 8) false)
        (`SceneComponent.SetVisibility` (`self.RenderComponent`) false false)
        (`SceneComponent.SetVisibility` (`self.PointLight`) false false)
        (set `self.isFireVisible` false)))))

(fn `UserConstructionScript`)