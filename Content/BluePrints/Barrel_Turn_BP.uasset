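; Barrel-turning actor that steers and cleans up spawned barrels as they pass through it.
; Overlapping its Trigger sets a tagged MyBarrelToSpawn's Rolly flag true, and leaving the Trigger clears it.
; A separate Death_box volume destroys any tagged barrel that overlaps it.
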(event `self.trigger.OnComponentBeginOverlap`
  (params (OverlappedComponent :type "PrimitiveComponent Object Reference") (OtherActor :type "Actor Object Reference") (OtherComp :type "PrimitiveComponent Object Reference") (OtherBodyIndex :type Integer) (bFromSweep :type Boolean) (SweepResult :type "HitResult Structure (by ref)"))
  (if (`self.ActorHasTag` OtherActor "Barrel")
    (bind _asmy_barrel_to_spawn (cast `/Game/BluePrints/MyBarrelToSpawn` OtherActor))
    (set `/Game/BluePrints/MyBarrelToSpawn.rolly` true _asmy_barrel_to_spawn)))

(event `self.trigger.OnComponentEndOverlap`
  (params (OverlappedComponent :type "PrimitiveComponent Object Reference") (OtherActor :type "Actor Object Reference") (OtherComp :type "PrimitiveComponent Object Reference") (OtherBodyIndex :type Integer))
  (if (`self.ActorHasTag` OtherActor "Barrel")
    (bind _asmy_barrel_to_spawn (cast `/Game/BluePrints/MyBarrelToSpawn` OtherActor))
    (set `/Game/BluePrints/MyBarrelToSpawn.rolly` false _asmy_barrel_to_spawn)))

(event `self.death_box.OnComponentBeginOverlap`
  (params (OverlappedComponent :type "PrimitiveComponent Object Reference") (OtherActor :type "Actor Object Reference") (OtherComp :type "PrimitiveComponent Object Reference") (OtherBodyIndex :type Integer) (bFromSweep :type Boolean) (SweepResult :type "HitResult Structure (by ref)"))
  (if (`self.ActorHasTag` OtherActor "Barrel")
    (bind _asmy_barrel_to_spawn (cast `/Game/BluePrints/MyBarrelToSpawn` OtherActor))
    (`self.K2_DestroyActor` _asmy_barrel_to_spawn)))

(fn `UserConstructionScript`)