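; A fall death volume that flags the player as dead when the player enters its Box.
; On overlap by an actor tagged Player, it casts player character 0 to PlayerController_BP and sets PlayerDead to the overlap's FromSweep flag, so it is true only for swept overlaps.
; The Box hit event casts without further effect, and disconnected leftover nodes, including one setting PlayerDead true, never run.
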(event `self.Box.OnComponentBeginOverlap`
  (params (OverlappedComponent :type "PrimitiveComponent Object Reference") (OtherActor :type "Actor Object Reference") (OtherComp :type "PrimitiveComponent Object Reference") (OtherBodyIndex :type Integer) (bFromSweep :type Boolean) (SweepResult :type "HitResult Structure (by ref)"))
  (if (`self.ActorHasTag` OtherActor "Player")
    (bind _asplayer_controller_bp (cast `/Game/BluePrints/PlayerController_BP` (`GameplayStatics.GetPlayerCharacter` 0)))
    (set `/Game/BluePrints/PlayerController_BP.playerDead` bFromSweep _asplayer_controller_bp)))

(event `self.ReceiveTick`
  (params (DeltaSeconds :type "Float (single-precision)")))

(event `self.Box.OnComponentHit`
  (params (HitComponent :type "PrimitiveComponent Object Reference") (OtherActor :type "Actor Object Reference") (OtherComp :type "PrimitiveComponent Object Reference") (NormalImpulse :type "Vector Structure") (Hit :type "HitResult Structure (by ref)"))
  (if (`self.ActorHasTag` OtherActor "Player")
    (cast `/Game/BluePrints/PlayerController_BP` (`GameplayStatics.GetPlayerCharacter` 0))))

(fn `UserConstructionScript`)