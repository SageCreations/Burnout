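; Barrel spawner that starts producing barrels when an actor tagged Player enters its box trigger.
; Tick spawns the barrel class at the sphere component's location, immediately at first, then about every two seconds via a Delay used as a repeat timer.
; Tick also casts the player character to PlayerController_BP and switches the spawner off while PlayerDead is set.
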(event `self.ReceiveTick`
  (params (DeltaSeconds :type "Float (single-precision)"))
  (bind _asplayer_controller_bp (cast `/Game/BluePrints/PlayerController_BP` (`GameplayStatics.GetPlayerCharacter` 0)))
  (if (`/Game/BluePrints/PlayerController_BP.playerDead` _asplayer_controller_bp)
    (set `self.activateSpawner` false)
    (elif (`self.activateSpawner`)
      (if (`self.firstTick`)
        (`KismetSystemLibrary.Delay` 2.0)
        (else
          (set `self.firstTick` true)))
      (`|SpawnActorFromClass` "/Game/BluePrints/MyBarrelToSpawn1.MyBarrelToSpawn1_C" (`KismetMathLibrary.Conv_VectorToTransform` (`SceneComponent.K2_GetComponentLocation` (`self.SphereComp`))) "Undefined" "OverrideRootScale" null null))))

(event `self.BoxComponent.OnComponentBeginOverlap`
  (params (OverlappedComponent :type "PrimitiveComponent Object Reference") (OtherActor :type "Actor Object Reference") (OtherComp :type "PrimitiveComponent Object Reference") (OtherBodyIndex :type Integer) (bFromSweep :type Boolean) (SweepResult :type "HitResult Structure (by ref)"))
  (if (`self.ActorHasTag` OtherActor "Player")
    (set `self.activateSpawner` true)))

(fn `UserConstructionScript`)